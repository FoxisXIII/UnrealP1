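; GameMode_BP is a game mode Blueprint that holds the game's Keys and Coins counters.
; Events add or spend keys one at a time, add or spend coins by a given value, and reset both totals, with no balance checks on spending.
; Getter functions expose both totals, and a Print Coins helper prints the new coin total after each coin add or spend.
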(event Custom|Add%20Key
  ;[1 1 1] Keys
  (Variables|Default|SetKeys (+ 1 (Variables|Default|GetKeys))))

(event Custom|SpendKeys
  ;[1 1 1] Keys
  (Variables|Default|SetKeys (- (Variables|Default|GetKeys) 1)))

(event Custom|Add%20Coins
  (params (Value :type Integer))
  ;[1 1 1] Coins
  (bind _output_get (Variables|Default|SetCoins (+ Value (Variables|Default|GetCoins))))
  (Utilities|PrintCoins (Utilities|String|ToString(Integer) _output_get)))

(event Custom|ResetAll
  (Variables|Default|SetKeys 0)
  (Variables|Default|SetCoins 0))

(event Custom|Spend%20Coins
  (params (Value :type Integer))
  ;[1 1 1] Coins
  (bind _output_get (Variables|Default|SetCoins (- (Variables|Default|GetCoins) Value)))
  (Utilities|PrintCoins (Utilities|String|ToString(Integer) _output_get)))

(fn ConstructionScript)

(fn GetCoins
  (return (Variables|Default|GetCoins)))

(fn GetKeys
  (return (Variables|Default|GetKeys)))