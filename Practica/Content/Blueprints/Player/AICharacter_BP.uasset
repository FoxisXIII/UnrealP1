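; AI character with a health bar that takes fixed damage per Die call and flags its death on the Blackboard.
; Each tick it turns the health widget toward the player and writes Life to the Blackboard.
; It can spawn an attached exclamation icon overhead with a given texture, and exposes attacking and healing state getters.
; DissolveObject drives a burn material effect with a timeline, then removes the widget and destroys the actor.
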(event Custom|Dissolve%20Object
  (bind _mesh (Variables|Character|GetMesh))
  ;[1 1 1] Dissolve
  (Rendering|Material|SetScalarParameterValueonMaterials _mesh "AllowBurn" 1.0)
  (bind _dissolution_value (Timeline|Dissolve Play)
    (:Update
      (Rendering|Material|SetScalarParameterValueonMaterials _mesh "DisolutionVal" _dissolution_value))
    (:Finished
      (bind _asai_wbp (Utilities|Casting|CastToAI_WBP (UserInterface|GetUserWidgetObject (Variables|Default|GetWidget))))
      (Widget|RemovefromParent _asai_wbp)
      (Actor|DestroyActor))))

(event Custom|Die
  ;[1 1 1] Hit/Die
  (if (> (Variables|Default|Getlife) 0.0)
    (Variables|Default|Setlife (- (Variables|Default|Getlife) 25.0))
    (CallFunction|UpdateLifeBar)
    (if (<= (Variables|Default|Getlife) 0.0)
      (Audio|PlaySoundatLocation "/Game/Sound/Damage.Damage" "0, 0, 0" "0, 0, 0" 1.0 1.0 0.0 0 0 0)
      (AI|Components|Blackboard|SetValueasBool (AI|GetBlackboard 0) (Utilities|Name|MakeLiteralName "Died") true))))

(event Custom|Exclamation
  (params (Texture :type Texture%202D%20Object%20Reference))
  ;[1 1 1] Sees Player
  (bind _returnvalue (Game|SpawnActorfromClass "/Game/Blueprints/AI/Exclamation_BP.Exclamation_BP_C" (Math|Transform|MakeTransform (+ (Transformation|GetActorLocation) (* (Transformation|GetActorUpVector) 200)) "0, 0, 0" "0.750000,0.750000,0.750000") "Undefined" 0 Texture 0))
  (Transformation|AttachActorToActor _returnvalue self "None" "KeepWorld" "SnapToTarget" "SnapToTarget" true))

(event EventTick
  (params (DeltaSeconds :type Float%20%28single-precision%29))
  ;[1 1 1] Look At
  (CallFunction|LookatPlayer)
  (AI|Components|Blackboard|SetValueasFloat (AI|GetBlackboard 0) (Utilities|Name|MakeLiteralName "Life") (Variables|Default|Getlife)))

(fn ConstructionScript)

(fn LookatPlayer
  (bind _widget (Variables|Default|GetWidget))
  (Transformation|SetWorldRotation _widget (Math|Rotator|FindLookatRotation (Transformation|GetWorldLocation _widget) (Transformation|GetWorldLocation (Variables|/Script/Engine.Character|GetCapsuleComponent (Game|GetPlayerCharacter 0)))) false false))

(fn UpdateLifeBar
  (bind _asai_wbp (Utilities|Casting|CastToAI_WBP (UserInterface|GetUserWidgetObject (Variables|Default|GetWidget))))
  (Default|SetHealth _asai_wbp (/ (Variables|Default|Getlife) (Variables|Default|GetmaxLife))))

(fn GetAttack
  (return (Variables|Default|GetAttacking)))

(fn GetHeal
  (return (Variables|Default|GetHealing)))