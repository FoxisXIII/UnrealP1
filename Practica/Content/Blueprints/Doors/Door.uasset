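; Sliding door actor that opens when an actor overlaps it and closes when the overlap ends.
; Overlap events set open and close flags, which Tick uses to move the Door along world Y at a constant, delta-time-scaled speed.
; Travel stops by comparing absolute Y values against the Trigger's Y recorded at BeginPlay, plus the YPosition distance for opening.
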(event Collision|EventActorBeginOverlap
  (params (OtherActor :type Actor%20Object%20Reference))
  (Variables|Default|SetCloseDoor false)
  (Variables|Default|SetOpenDoor true))

(event Collision|EventActorEndOverlap
  (params (OtherActor :type Actor%20Object%20Reference))
  (Variables|Default|SetCloseDoor true)
  (Variables|Default|SetOpenDoor false))

(event EventBeginPlay
  (Variables|Default|SetInitialYPosition (.y (.location (Transformation|GetWorldTransform (Variables|Default|GetTrigger))))))

(event EventTick
  (params (DeltaSeconds :type Float%20%28single-precision%29))
  (if (Variables|Default|GetOpenDoor)
    (CallFunction|Open)
    (elif (Variables|Default|GetCloseDoor)
      (CallFunction|Close))))

(fn ConstructionScript)

(fn Open
  (bind _door (Variables|Default|GetDoor))
  (bind _returnvalue (Transformation|GetWorldLocation _door))
  (if (> (+ (Math|Float|Absolute(Float) (Variables|Default|GetYPosition)) (Math|Float|Absolute(Float) (Variables|Default|GetInitialYPosition))) (Math|Float|Absolute(Float) (.y (Transformation|GetWorldLocation (Variables|Default|GetDoor)))))
    (Transformation|SetWorldLocation _door (Math|Vector|MakeVector (.x _returnvalue) (+ (.y _returnvalue) (* (Utilities|Time|GetWorldDeltaSeconds) 1e+02)) (.z _returnvalue)) false false)
    (else
      (Variables|Default|SetOpenDoor false))))

(fn Close
  (bind _door (Variables|Default|GetDoor))
  (bind _returnvalue (Transformation|GetWorldLocation _door))
  (if (< (Math|Float|Absolute(Float) (Variables|Default|GetInitialYPosition)) (Math|Float|Absolute(Float) (.y (Transformation|GetWorldLocation (Variables|Default|GetDoor)))))
    (Transformation|SetWorldLocation _door (Math|Vector|MakeVector (.x _returnvalue) (- (.y _returnvalue) (* (Utilities|Time|GetWorldDeltaSeconds) 1e+02)) (.z _returnvalue)) false false)
    (else
      (Variables|Default|SetCloseDoor false))))