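; Puzzle door, a child Blueprint that only passes begin overlap to its parent's door logic when three light bulbs all match a solution color sequence.
; GetLightX compares one bulb's RGB to the Solution entry at that index and branches True or False.
; Every Tick, three point lights show green or red for each position's match.
; End overlap always passes through to the parent.
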(event Collision|EventActorEndOverlap
  (params (OtherActor :type Actor%20Object%20Reference))
  (|CallParentFunction OtherActor))

(event Collision|EventActorBeginOverlap
  (params (OtherActor :type Actor%20Object%20Reference))
  (Utilities|GetLightX
    (:True
      (Utilities|GetLightX 1
        (:True
          (Utilities|GetLightX 2
            (:True
              (|CallParentFunction OtherActor))))))))

(event EventTick
  (params (DeltaSeconds :type Float%20%28single-precision%29))
  (Utilities|GetLightX
    (:True
      (Rendering|Components|Light|SetLightColor (Variables|Default|GetPointLight%20%281%29) "(R=0.000000,G=1.000000,B=0.000000,A=1.000000)" true))
    (:False
      (Rendering|Components|Light|SetLightColor (Variables|Default|GetPointLight%20%281%29) "(R=1.000000,G=0.000000,B=0.000000,A=1.000000)" true)))
  (Utilities|GetLightX 1
    (:True
      (Rendering|Components|Light|SetLightColor (Variables|Default|GetPointLight%20%282%29) "(R=0.000000,G=1.000000,B=0.000000,A=1.000000)" true))
    (:False
      (Rendering|Components|Light|SetLightColor (Variables|Default|GetPointLight%20%282%29) "(R=1.000000,G=0.000000,B=0.000000,A=1.000000)" true)))
  (Utilities|GetLightX 2
    (:True
      (Rendering|Components|Light|SetLightColor (Variables|Default|GetPointLight%20%283%29) "(R=0.000000,G=1.000000,B=0.000000,A=1.000000)" true))
    (:False
      (Rendering|Components|Light|SetLightColor (Variables|Default|GetPointLight%20%283%29) "(R=1.000000,G=0.000000,B=0.000000,A=1.000000)" true)))
  (|CallParentFunction DeltaSeconds))

(fn ConstructionScript
  (|CallParentFunction))