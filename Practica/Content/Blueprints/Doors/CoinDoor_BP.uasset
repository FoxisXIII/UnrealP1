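; CoinDoor_BP is a door that charges coins before it opens, inheriting its overlap behavior from a parent Blueprint.
; On first overlap it checks the coin count in GameMode_BP, spends the required Coins and sets Paid, or prints how many coins are needed.
; The parent's begin-overlap logic runs only once paid, so later overlaps pass straight through, while end-overlap always forwards to the parent.
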(event Collision|EventActorBeginOverlap
  (params (OtherActor :type Actor%20Object%20Reference))
  (if (Variables|Default|GetPaid)
    (|CallParentFunction OtherActor :!label _label)
    (else
      (bind _asgame_mode_bp (Utilities|Casting|CastToGameMode_BP (Game|GetGameMode)))
      (bind _coins (Default|GetCoins _asgame_mode_bp))
      (if (>= _coins (Variables|Default|GetCoins))
        (Default|SpendCoins _asgame_mode_bp (Variables|Default|GetCoins))
        (Variables|Default|SetPaid true)
        (goto _label)
        (else
          (Development|PrintString (Utilities|String|Append "You need " (Utilities|String|ToString(Integer) (Variables|Default|GetCoins)) " Coins") true true "(R=1.000000,G=0.000000,B=0.000000,A=1.000000)"))))))

(event EventTick
  (params (DeltaSeconds :type Float%20%28single-precision%29))
  (|CallParentFunction DeltaSeconds) ; This node is disabled and will not be called.\nDrag off pins to build functionality.
)

(event Collision|EventActorEndOverlap
  (params (OtherActor :type Actor%20Object%20Reference))
  (|CallParentFunction OtherActor))

(fn ConstructionScript
  (|CallParentFunction))