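; Door_BP is a sliding door actor that opens when another actor begins overlapping it and closes when the overlap ends.
; Overlap events set OpenDoor and CloseDoor flags, which Tick reads to call Open or Close.
; These move the whole actor along its forward vector at delta-scaled speed, but limit travel with a per-tick Counter against YPosition, so distance depends on frame rate.
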(event EventBeginPlay
  (Development|PrintString (Utilities|String|ToString(Vector) (Math|Vector|GetForwardVector (Variables|Default|GetArrow)))))

(event Collision|EventActorBeginOverlap
  (params (OtherActor :type Actor%20Object%20Reference))
  (Variables|Default|SetCloseDoor false)
  (Variables|Default|SetOpenDoor true))

(event Collision|EventActorEndOverlap
  (params (OtherActor :type Actor%20Object%20Reference))
  (Variables|Default|SetCloseDoor true)
  (Variables|Default|SetOpenDoor false))

(event EventTick
  (params (DeltaSeconds :type Float%20%28single-precision%29))
  (if (Variables|Default|GetOpenDoor)
    (CallFunction|Open)
    (elif (Variables|Default|GetCloseDoor)
      (CallFunction|Close))))

(fn ConstructionScript)

(fn Open
  (if (<= (Variables|Default|GetCounter) (Variables|Default|GetYPosition))
    (Math|Float|IncrementFloat (Variables|Default|GetCounter)
      (:%20%20
        (Transformation|SetActorLocation (+ (* (Transformation|GetActorForwardVector) (* (Utilities|Time|GetWorldDeltaSeconds) 1e+02)) (Transformation|GetActorLocation)) false false)))
    (else
      (Variables|Default|SetOpenDoor false))))

(fn Close
  (if (> (Variables|Default|GetCounter) 0.0)
    (Math|Float|DecrementFloat (Variables|Default|GetCounter)
      (:%20%20
        (Transformation|SetActorLocation (+ (* (Transformation|GetActorForwardVector) (* (Utilities|Time|GetWorldDeltaSeconds) -1e+02)) (Transformation|GetActorLocation)) false false)))
    (else
      (Variables|Default|SetOpenDoor false))))