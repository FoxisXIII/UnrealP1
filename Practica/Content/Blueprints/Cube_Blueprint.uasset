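; Cube Blueprint is an actor that acts as a vertical moving platform, shuttling between its start position and a point 1000 units above it.
; Each Tick, MovePlatform offsets it along the up vector at a fixed speed scaled by delta time, without sweep.
; On reaching either limit it flips direction and MantainPlatform holds it there for about five seconds using an accumulated timer.
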(event EventBeginPlay
  (bind _output_get (Variables|Default|SetminPos (Transformation|GetActorLocation)))
  (Variables|Default|SetmaxPos (Math|Vector|MakeVector (.x _output_get) (.y _output_get) (+ (.z _output_get) 1e+03)))
  (Variables|Default|SetmovingUp true)
  (Variables|Default|SetMantain false))

(event Collision|EventActorBeginOverlap
  (params (OtherActor :type Actor%20Object%20Reference)))

(event EventTick
  (params (DeltaSeconds :type Float%20%28single-precision%29))
  (if (Variables|Default|GetMantain)
    (CallFunction|MantainPlatform)
    (else
      (if (Variables|Default|GetmovingUp)
        (Variables|Default|SetDirection 5e+02)
        (else
          (Variables|Default|SetDirection -5e+02)))
      (CallFunction|MovePlatform))))

(fn ConstructionScript)

(fn MovePlatform
  (if (Variables|Default|GetmovingUp)
    (if (>= (.z (Transformation|GetActorLocation)) (.z (Variables|Default|GetmaxPos)))
      (Variables|Default|SetMantain true)
      (Variables|Default|SetmovingUp false)
      (Variables|Default|Setcounter 0.0)
      (else
        (Transformation|SetActorLocation (+ (Transformation|GetActorLocation) (* (Math|Vector|VectorUp) (* (Utilities|Time|GetWorldDeltaSeconds) (Variables|Default|GetDirection)))) false false :!label _label)))
    (elif (<= (.z (Transformation|GetActorLocation)) (.z (Variables|Default|GetminPos)))
      (Variables|Default|SetMantain true)
      (Variables|Default|SetmovingUp true)
      (Variables|Default|Setcounter 0.0)
      (else
        (goto _label)))))

(fn MantainPlatform
  (bind _output_get (Variables|Default|Setcounter (+ (Utilities|Time|GetWorldDeltaSeconds) (Variables|Default|Getcounter))))
  (if (> _output_get 5.0)
    (Variables|Default|SetMantain false)))