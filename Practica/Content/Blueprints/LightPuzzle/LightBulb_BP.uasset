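; LightBulb_BP is a puzzle light bulb whose point light color the player can change by pressing 1 while overlapping it.
; Overlap events maintain an IsColliding flag through a player pawn check, though the on-screen prompt shows for any overlapping actor and any actor leaving clears the flag.
; ChangeLightColor applies the current LightsColors entry, then advances a counter that wraps around at the end of the array.
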(event Collision|EventActorBeginOverlap
  (params (OtherActor :type Actor%20Object%20Reference))
  (CallFunction|CollisionwithPlayer OtherActor)
  (Development|PrintString "Press 1 to change the light color" true true "(R=1.000000,G=1.000000,B=0.000000,A=1.000000)"))

(event Collision|EventActorEndOverlap
  (params (OtherActor :type Actor%20Object%20Reference))
  (CallFunction|CollisionwithPlayer OtherActor)
  (Variables|Default|SetIsColliding false))

(event Input|KeyboardEvents|1
  (params (Key :type Key%20Structure :default "None"))
  (:Pressed
    (CallFunction|ChangeLightColor)))

(fn ConstructionScript)

(fn ChangeLightColor
  (if (Variables|Default|GetIsColliding)
    (Rendering|Components|Light|SetLightColor (Variables|Default|GetPointLightComponent) (Utilities|Array|Get(acopy) (Variables|Default|GetLights%20Colors) (Variables|Default|GetCounter)) true)
    (if (< (Variables|Default|GetCounter) (- (Utilities|Array|Length (Variables|Default|GetLights%20Colors)) 1))
      (Math|Integer|IncrementInt (Variables|Default|GetCounter))
      (else
        (Variables|Default|SetCounter 0)))))

(fn CollisionwithPlayer
  (params (A :type Object%20Object%20Reference))
  (if (== A (Game|Player|GetPlayerPawn 0))
    (bind _output_get (Variables|Default|SetIsColliding true))
    (Development|PrintString (Utilities|String|ToString(Boolean) (Variables|Default|GetIsColliding)) _output_get)))